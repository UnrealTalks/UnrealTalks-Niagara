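; BP_Galton is a Galton board actor that procedurally lays out a field of pegs with a row of bin dividers at one end.
; The Construction Script loops over a centered X/Y grid sized by PegNumX, PegNumY and Spacing, adding instances to PegInstance and Dividers.
; Odd peg rows shift by half the spacing, with a sign multiply keeping the stagger consistent across negative indices.
; The Event Graph holds no runtime logic.
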(event EventBeginPlay)

(event Collision|EventActorBeginOverlap
  (params (OtherActor :type Actor%20Object%20Reference)))

(event EventTick
  (params (DeltaSeconds :type Float%20%28single-precision%29)))

(fn ConstructionScript
  (bind _spacing (Variables|Default|GetSpacing))
  (bind _spacing_2 (Variables|Default|GetSpacing))
  (bind _pegsize (Variables|Default|GetPegSize))
  (bind _pegnumx (Variables|Default|GetPegNumX))
  (bind _pegnumy (Variables|Default|GetPegNumY))
  (for _index (range (* _pegnumx -1) _pegnumx)
    (Components|InstancedStaticMesh|AddInstance (Variables|Default|GetDividers) (Math|Transform|MakeTransform (Math|Vector|MakeVector (* _index _spacing) (- (* (Variables|Default|GetPegNumY) _spacing) -1e+01) 0.0) "0, 0, 0" "1,20.000000,10.000000"))
    (for _index_2 (range (* _pegnumy -1) _pegnumy)
      (Components|InstancedStaticMesh|AddInstance (Variables|Default|GetPegInstance) (Math|Transform|MakeTransform (Math|Vector|MakeVector (+ (* (Class|KismetMathLibrary|SignOfInteger _index_2) (* (Math|Integer|%(Integer) _index_2 2) (/ _spacing_2 2.0))) (* _index _spacing_2)) (* _index_2 _spacing_2) 0.0) "0, 0, 0" (Math|Vector|MakeVector _pegsize _pegsize 0.15))))))